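; Player controller for a team-based "Strike" mode that shows the team selection UI on BeginPlay.
; ShowHideWidget forwards a widget identifier and show flag to a CL-prefixed event, which calls the show or hide function.
; Those functions switch on the widget, lazily creating and caching the team selection widget before adding it to the viewport, or removing it from its parent.
; A helper function returns the controller itself.
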(event Custom|ShowHideWidget
  (params (Widget :type E_GameWidget%20Enum :default "NewEnumerator0") (bShow :type Boolean))
  ;[1 0 0.6038] UIを見せるか見せないかの処理
  (CallFunction|CLShowHideWidget Widget bShow))

(event Custom|CL_ShowHideWidget
  (params (Widget :type E_GameWidget%20Enum :default "NewEnumerator0") (bShow :type Boolean))
  ;[1 0 0.6038] UIを見せるか見せないかの処理
  (if bShow
    (CallFunction|FShowWidget (Variables|Default|GetWidget))
    (else
      (CallFunction|FHideWidget (Variables|Default|GetWidget)))))

(event EventBeginPlay
  ;[1 0 0.6038] UIを見せるか見せないかの処理
  (CallFunction|ShowHideWidget "NewEnumerator0" true))

(fn ConstructionScript)

(fn FShowWidget
  (params (Widget :type E_GameWidget%20Enum :default "NewEnumerator0"))
  (switch Utilities|FlowControl|Switch|SwitchonE_GameWidget Widget
    (:NewEnumerator0
      (Variables|Default|GetWB_TeamSelection
        (:then
          _)
        (:else
          (bind _returnvalue (UserInterface|CreateWidget "/Game/UI/WB_TeamSelection.WB_TeamSelection_C"))
          (bind _output_get (Variables|Default|SetWB_TeamSelection _returnvalue))))
      (UserInterface|Viewport|AddtoViewport _output_get 0))))

(fn FHideWidget
  (params (Widget :type E_GameWidget%20Enum :default "NewEnumerator0"))
  (switch Utilities|FlowControl|Switch|SwitchonE_GameWidget Widget
    (:NewEnumerator0
      (bind _wb_teamselection (Variables|Default|GetWB_TeamSelection)
        (:then
          (Widget|RemovefromParent _wb_teamselection))
        (:else)))))

(fn GetPlayerControllerRef
  (return self))