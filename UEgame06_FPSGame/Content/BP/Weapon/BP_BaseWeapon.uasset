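; Base weapon actor that simulates physics and acts as a world pickup for players.
; On the server, sphere overlap selects an interacting player, skipping their just-dropped weapon, and registers itself with them unless their inventory holds the same weapon type.
; If the weapon is not yet interactable, the check retries on a short delay.
; Leaving the sphere calls SetDroppedWeapon on that player, and GetWeaponRef returns the weapon itself.
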(event OnComponentBeginOverlap(CollisionSphere)
  (params (OverlappedComponent :type Primitive%20Component%20Object%20Reference) (OtherActor :type Actor%20Object%20Reference) (OtherComp :type Primitive%20Component%20Object%20Reference) (OtherBodyIndex :type Integer) (bFromSweep :type Boolean) (SweepResult :type Hit%20Result%20Structure%20%28by%20ref%29))
  (bind _overlappingactors (Collision|GetOverlappingActors "/Game/BP/Player/BP_PlayerBase.BP_PlayerBase_C" :!class /Script/Engine.Actor))
  (if (Actor|ActorHasTag OtherActor "Player")
    (Networking|SwitchHasAuthority
      (:Authority
        (if (Variables|Default|GetbCanbeInteractedWith) :!label _label
          (if (> (Utilities|Array|Length _overlappingactors) 1)
            (bind _array_element (Utilities|Array|ForEachLoopwithBreak _overlappingactors :!label _label_2)
              (:LoopBody
                (bind _player (Class|ITFPlayerBase|GetPlayerRef(Message) _array_element))
                (if (!= (Variables|/Game/BP/Player/BP_PlayerBase.BP_PlayerBase_C|GetDropped%20Weapon _player) self)
                  (Variables|Default|SetInteractingPlayer _player)
                  (goto _label_2 Break)))
              (:Completed
                (bind _array_element_2 (Utilities|Array|ForEachLoopwithBreak (Variables|/Game/BP/Player/BP_PlayerBase.BP_PlayerBase_C|GetWeaponInventory (Variables|Default|GetInteractingPlayer)) :!label _label_3)
                  (:LoopBody
                    (if (Utilities|Enum|Equal(Enum) (.type (Utilities|Struct|BreakST_WeaponInfo (CallFunction|FGetWeaponInfo (Variables|BP_BaseWeapon_C|GetWeaponName _array_element_2)))) (.type (Utilities|Struct|BreakST_WeaponInfo (CallFunction|FGetWeaponInfo (Variables|Default|GetWeaponName)))))
                      (Variables|/Game/BP/Player/BP_PlayerBase.BP_PlayerBase_C|SetbCanLootWeapon (Variables|Default|GetInteractingPlayer) false)
                      (goto _label_3 Break)))
                  (:Completed
                    (if (Variables|/Game/BP/Player/BP_PlayerBase.BP_PlayerBase_C|GetbCanLootWeapon (Variables|Default|GetInteractingPlayer))
                      (Default|AddOverlappedWeapon (Variables|Default|GetInteractingPlayer) self)
                      (else
                        (Variables|/Game/BP/Player/BP_PlayerBase.BP_PlayerBase_C|SetbCanLootWeapon (Variables|Default|GetInteractingPlayer) true)))))))
            (else
              (bind _player_2 (Class|ITFPlayerBase|GetPlayerRef(Message) (Utilities|Array|Get(acopy) _overlappingactors)))
              (bind _output_get (Variables|Default|SetInteractingPlayer _player_2))
              (if (!= (Variables|/Game/BP/Player/BP_PlayerBase.BP_PlayerBase_C|GetDropped%20Weapon _output_get) self)
                (goto _label_3))))
          (else
            (Utilities|FlowControl|Delay 0.1)
            (goto _label)))))))

(event OnComponentEndOverlap(CollisionSphere)
  (params (OverlappedComponent :type Primitive%20Component%20Object%20Reference) (OtherActor :type Actor%20Object%20Reference) (OtherComp :type Primitive%20Component%20Object%20Reference) (OtherBodyIndex :type Integer))
  (if (Actor|ActorHasTag OtherActor "Player")
    (Networking|SwitchHasAuthority
      (:Authority
        (bind _player (Class|ITFPlayerBase|GetPlayerRef(Message) OtherActor))
        (Default|SetDroppedWeapon _player)))))

(event EventBeginPlay
  ;[0.123 0 1] Begin Play
  (Physics|SetSimulatePhysics (Variables|Default|GetWeapon) true))

(fn ConstructionScript)

(fn GetWeaponRef
  (return self))