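; Game mode for a team shooter that tracks connected players and picks spawn locations for Counter-Terrorist and Terrorist teams.
; On PostLogin it records the new player and gathers each team's spawn actors by class.
; RequestSpawnPlayer selects a random transform from the requested team's list and passes it with the team to the controller's SpawnPlayer.
; GetGameModeRef returns the game mode itself.
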(event Custom|RequestSpawnPlayer
  (params (PlayerController :type PC%20Controller%20Strike%20Object%20Reference) (Team :type Actor%20Class%20Reference))
  (Default|SpawnPlayer PlayerController Team (Math|Transform|SelectTransform (Transformation|GetActorTransform (.OutItem (Utilities|Array|Random (Variables|Default|GetCounterTerroristSpawnPoint)))) (Transformation|GetActorTransform (.OutItem (Utilities|Array|Random (Variables|Default|GetTerroristSpawnPoint)))) (== Team "/Game/BP/Player/BP_CounterTerrorist.BP_CounterTerrorist_C"))))

(event EventPostLogin
  (params (NewPlayer :type Player%20Controller%20Object%20Reference))
  (Utilities|Array|AddUnique (Variables|Default|GetConnectedPlayers) NewPlayer)
  (bind _outactors (Actor|GetAllActorsOfClass "/Game/BP/Player/BP_CounterTerrorist.BP_CounterTerrorist_C"))
  (Variables|Default|SetCounterTerroristSpawnPoint _outactors)
  (bind _outactors_2 (Actor|GetAllActorsOfClass "/Game/BP/Player/SpawnPoint/BP_TeroristSpawnPoint.BP_TeroristSpawnPoint_C"))
  (Variables|Default|SetTerroristSpawnPoint _outactors_2))

(fn ConstructionScript)

(fn GetGameModeRef
  (return self))